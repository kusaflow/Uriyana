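; Breakable small-width glass pane that shatters when hit by a ThrowBall actor.
; On such a hit, the Destructible component takes radius damage with an impulse at the impact point.
; If the PlaneGlass component is still valid, it is destroyed and gravity is enabled on the Destructible.
; Tick also sets the Box component to a hardcoded world location every frame.
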(event OnComponentHit(Destructible)
  (params (HitComponent :type Primitive%20Component%20Object%20Reference) (OtherActor :type Actor%20Object%20Reference) (OtherComp :type Primitive%20Component%20Object%20Reference) (NormalImpulse :type Vector :default "0, 0, 0") (Hit :type Hit%20Result%20Structure%20%28by%20ref%29))
  (Utilities|Casting|CastToThrowBall OtherActor)
  (Class|DestructibleComponent|ApplyRadiusDamage (Variables|Default|GetDestructible) 6e+04 (.Location (Collision|BreakHitResult Hit)) 2e+02 5e+03 true)
  (Utilities|IsValid (Variables|Default|GetplaneGlass)
    (:Is%20Valid
      (Components|DestroyComponent (Variables|Default|GetplaneGlass))
      (Physics|SetEnableGravity (Variables|Default|GetDestructible) true))))

(event EventBeginPlay)

(event Collision|EventActorBeginOverlap
  (params (OtherActor :type Actor%20Object%20Reference)))

(event EventTick
  (params (DeltaSeconds :type Float%20%28single-precision%29))
  (Transformation|SetWorldLocation (Variables|Default|GetBox) "0.000000,400.000000,1000.000000" false false))

(fn ConstructionScript)