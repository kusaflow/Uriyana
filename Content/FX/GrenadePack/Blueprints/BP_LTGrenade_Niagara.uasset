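; Grenade projectile actor that explodes after a random short fuse, with Niagara effects matched to the surface beneath it.
; A short downward trace picks the effect by the physical material's surface type, or an air burst when nothing is hit.
; The blast then adds a randomized fading scorch decal, light flash, camera shake, radial damage, force impulse and sound, and hides the grenade.
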(event EventBeginPlay
  (bind _decalscalemin (Variables|Default|GetDecalScaleMin))
  (bind _spherecollision (Variables|Default|GetSphereCollision))
  (bind _decalrotationmin (Variables|Default|GetDecalRotationMin))
  (bind _decalrotationmax (Variables|Default|GetDecalRotationMax))
  (bind _decalscalemax (Variables|Default|GetDecalScaleMax))
  (bind _returnvalue (Math|Random|RandomFloatinRange _decalscalemin _decalscalemax))
  (bind _returnvalue_2 (Transformation|GetWorldLocation _spherecollision))
  (bind _returnvalue_3 (Math|Random|RandomFloatinRange _decalrotationmin _decalrotationmax))
  ;[1 1 1] Grenade Projectile Info
  (Variables|Default|SetGrenadeListNiagara (Utilities|Array|MakeArray (Variables|Default|GetNSDefault) (Variables|Default|GetNSConcrete) (Variables|Default|GetNSDirt) (Variables|Default|GetNSGrass) (Variables|Default|GetNSIce) (Variables|Default|GetNSMetal) (Variables|Default|GetNSSand) (Variables|Default|GetNSSnow) (Variables|Default|GetNSWater) (Variables|Default|GetNS_Wood)))
  (Variables|Default|SetFuseTime (Math|Random|RandomFloatinRange 1.0 2.0))
  (Variables|Default|SetArmed true)
  (Utilities|FlowControl|Delay (Variables|Default|GetFuseTime))
  (bind (_outhit _returnvalue_4) (Collision|LineTraceByChannel _returnvalue_2 (+ _returnvalue_2 "0, 0,-100.000000") "TraceTypeQuery1" false 0 "None"))
  (if _returnvalue_4
    (Niagara|SpawnSystematLocation (Utilities|Array|Get(acopy) (Variables|Default|GetGrenadeListNiagara) (Math|Conversions|ToInteger(Byte) (Variables|/Script/Engine.PhysicalMaterial|GetSurfaceType (.PhysMat (Collision|BreakHitResult _outhit))))) (.Location (Collision|BreakHitResult _outhit)) (Math|Rotator|MakeRotationfromAxes (.Normal (Collision|BreakHitResult _outhit)) "0, 0, 0" "0, 0, 0"))
    (else
      (Niagara|SpawnSystematLocation (Variables|Default|GetAirNiagara) _returnvalue_2)))
  (bind _returnvalue_5 (Rendering|Decal|SpawnDecalatLocation "/Game/FX/GrenadePack/Materials/M_scorch.M_scorch" (Math|Vector|MakeVector _returnvalue _returnvalue _returnvalue) (.Location (Collision|BreakHitResult _outhit)) (Math|Rotator|MakeRotator _returnvalue_3 -9e+01 _returnvalue_3) 0.0))
  (Development|SetHiddeninGame (Variables|Default|GetStaticMesh1) true false)
  (Rendering|Components|Decal|SetFadeOut _returnvalue_5 (Variables|Default|GetDecal%20Start%20Delay) (Variables|Default|GetDecalLife) true)
  (Rendering|ToggleVisibility (Variables|Default|GetPointLight) false)
  (Utilities|FlowControl|Delay 0.2)
  (Rendering|ToggleVisibility (Variables|Default|GetPointLight) false)
  (Rendering|SetActorHiddenInGame true)
  (Camera|PlayWorldCameraShake (Variables|Default|GetCameraShake) (.Location (Collision|BreakHitResult _outhit)) 0.0 2e+03)
  (Game|Damage|ApplyRadialDamage 2e+02 (.Location (Collision|BreakHitResult _outhit)) 1e+02 0 0 0 0 false "ECC_Visibility")
  (Utilities|FlowControl|DoOnce false
    (:Completed
      (Class|RadialForceComponent|FireImpulse (Variables|Default|GetRadialForce1))
      (Audio|SpawnSoundAttached "/Game/FX/GrenadePack/MapAssets/Audio/Explosion01.Explosion01" _returnvalue_5 "None" "0, 0, 0" "0, 0, 0" "KeepRelativeOffset" false 1.0 1.0 0.0 0 0))))

(fn ConstructionScript)