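; Grenade projectile actor that explodes after a short random fuse, with effects that depend on the surface beneath it.
; A downward trace uses the physical surface type to index an emitter array, falling back to an air burst on a miss.
; The blast spawns a randomized fading scorch decal, toggles a brief light, hides the grenade and triggers camera shake, radial damage, a physics impulse and sound.
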(event EventBeginPlay
  (bind _decalrotationmin (Variables|Default|GetDecalRotationMin))
  (bind _decalrotationmax (Variables|Default|GetDecalRotationMax))
  (bind _decalscalemin (Variables|Default|GetDecalScaleMin))
  (bind _decalscalemax (Variables|Default|GetDecalScaleMax))
  (bind _spherecollision (Variables|Default|GetSphereCollision))
  (bind _decal_life (Variables|Default|GetDecal%20Life))
  (bind _returnvalue (Transformation|GetWorldLocation _spherecollision))
  (bind _returnvalue_2 (Math|Random|RandomFloatinRange _decalrotationmin _decalrotationmax))
  (bind _returnvalue_3 (Math|Random|RandomFloatinRange _decalscalemin _decalscalemax))
  ;[1 1 1] Grenade Projectile Info
  (Variables|Default|SetGrenadeList (Utilities|Array|MakeArray (Variables|VFX|GetDefault) (Variables|VFX|GetConcrete) (Variables|VFX|GetDirt) (Variables|VFX|GetGrass) (Variables|VFX|GetIce) (Variables|VFX|GetMetal) (Variables|VFX|GetSand) (Variables|VFX|GetSnow) (Variables|VFX|GetWater) (Variables|VFX|GetWood)))
  (Variables|Default|SetFuseTime (Math|Random|RandomFloatinRange 1.0 2.0))
  (Variables|Default|SetArmed true)
  (Utilities|FlowControl|Delay (Variables|Default|GetFuseTime))
  (bind (_outhit _returnvalue_4) (Collision|LineTraceByChannel _returnvalue (+ _returnvalue "0, 0,-100.000000") "TraceTypeQuery1" false 0 "None"))
  (if _returnvalue_4
    (Effects|SpawnEmitteratLocation (Utilities|Array|Get(acopy) (Variables|Default|GetGrenadeList) (Math|Conversions|ToInteger(Byte) (Variables|/Script/Engine.PhysicalMaterial|GetSurfaceType (.PhysMat (Collision|BreakHitResult _outhit))))) (.Location (Collision|BreakHitResult _outhit)) (Math|Rotator|MakeRotationfromAxes (.Normal (Collision|BreakHitResult _outhit)) "0, 0, 0" "0, 0, 0"))
    (else
      (Effects|SpawnEmitteratLocation (Variables|VFX|GetAir) _returnvalue)))
  (bind _returnvalue_5 (Rendering|Decal|SpawnDecalatLocation "/Game/FX/GrenadePack/Materials/M_scorch.M_scorch" (Math|Vector|MakeVector _returnvalue_3 _returnvalue_3 _returnvalue_3) (.Location (Collision|BreakHitResult _outhit)) (Math|Rotator|MakeRotator _returnvalue_2 -9e+01 _returnvalue_2) _decal_life))
  (Development|SetHiddeninGame (Variables|Default|GetStaticMesh1) true false)
  (Rendering|Components|Decal|SetFadeOut _returnvalue_5 (Variables|Default|GetDecal%20Start%20Delay) _decal_life true)
  (Rendering|ToggleVisibility (Variables|Default|GetPointLight) false)
  (Utilities|FlowControl|Delay 0.2)
  (Rendering|ToggleVisibility (Variables|Default|GetPointLight) false)
  (Rendering|SetActorHiddenInGame true)
  (Camera|PlayWorldCameraShake (Variables|Default|GetCameraShake) (.Location (Collision|BreakHitResult _outhit)) 0.0 2e+03)
  (Game|Damage|ApplyRadialDamage 2e+02 (.Location (Collision|BreakHitResult _outhit)) 1e+02 0 0 0 0 false "ECC_Visibility")
  (Utilities|FlowControl|DoOnce false
    (:Completed
      (Class|RadialForceComponent|FireImpulse (Variables|Default|GetRadialForce1))
      (Audio|SpawnSoundAttached "/Game/FX/GrenadePack/MapAssets/Audio/Explosion01.Explosion01" _returnvalue_5 "None" "0, 0, 0" "0, 0, 0" "KeepRelativeOffset" false 1.0 1.0 0.0 0 0))))

(fn ConstructionScript)