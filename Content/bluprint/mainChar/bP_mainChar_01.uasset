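; Main character Blueprint that sets up the on-screen UI and offers a key to refill gun stamina.
; On BeginPlay it creates the UI_MG widget and adds it to the viewport.
; Pressing K adds a fixed amount to CurrentGunStamina on kusaGameInstance, with no clamp in this graph.
; A print of that stamina value is left unconnected, and Tick and construction script are empty.
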(event EventBeginPlay
  (bind _returnvalue (UserInterface|CreateWidget "/Game/bluprint/mainChar/UI_MG.UI_MG_C"))
  (UserInterface|Viewport|AddtoViewport _returnvalue 0))

(event Collision|EventActorBeginOverlap
  (params (OtherActor :type Actor%20Object%20Reference)))

(event EventTick
  (params (DeltaSeconds :type Float%20%28single-precision%29)))

(event Input|KeyboardEvents|K
  (params (Key :type Key%20Structure :default "None"))
  (:Pressed
    (bind _askusa_game_instance (Utilities|Casting|CastTokusaGameInstance (Game|GetGameInstance)))
    (Variables|/Script/Uriyana.kusaGameInstance|SetCurrentGunStamina _askusa_game_instance (+ (Variables|/Script/Uriyana.kusaGameInstance|GetCurrentGunStamina _askusa_game_instance) 1e+02))))

(fn ConstructionScript)